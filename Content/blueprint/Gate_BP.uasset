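; Gate_BP is an interactable double gate that stays shut while locked.
; OpendoorF clears the lock when it receives a true AllBattery flag, meaning the player has all batteries.
; Interact calls OpenDoor if unlocked, which plays a timeline that lerps the left and right gate yaw 90 degrees in opposite directions.
; The gate has no closing logic.
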(event `Open Door`
  ;[1 1 1] Gate open animatiion
  (if (not (`self.Isdoorlocked?`))
    (bind (_direction _door_opentrack) (`Timeline|door open timeline`)
      (:`Update`
        (`SceneComponent.K2_SetRelativeRotation` (`self.RightGate`) (`KismetMathLibrary.MakeRotator` 0.0 0.0 (`KismetMathLibrary.Lerp` 0.0 90.0 _door_opentrack)) false false)
        (`SceneComponent.K2_SetRelativeRotation` (`self.LeftGate`) (`KismetMathLibrary.MakeRotator` 0.0 0.0 (`KismetMathLibrary.Lerp` 0.0 -90.0 _door_opentrack)) false false)))))

(event `/Game/blueprint/InteractInterface.Opendoor_f`
  (params (`all battery?` :type Boolean))
  ;[1 1 1] you get all battery
  (if `all battery?`
    (set `self.Isdoorlocked?` false)))

(event `/Game/blueprint/InteractInterface.Interact`
  (params (fpscharacter :type "/Game/blueprint/fpscharacter_BP Object Reference"))
  ;[1 1 1] Open Door
  (if (not (`self.Isdoorlocked?`))
    (`self.Open Door`)))

(fn `UserConstructionScript`)
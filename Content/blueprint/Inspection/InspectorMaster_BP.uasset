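; Base inspectable item actor that the player examines up close, picks up, or uses from the inventory.
; Inspection attaches it in front of the camera, shows an item widget and moves input from the character to the item.
; Right click collects it, stacking duplicates, with name-matched special cases for the flashlight and colored batteries.
; When opened from inventory, it instead supports using the item or closing the inventory, destroying the actor afterwards.
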(event `/Game/blueprint/InteractInterface.Interact`
  (params (fpscharacter :type "/Game/blueprint/fpscharacter_BP Object Reference"))
  ;[1 1 1] If press E -> Inspect
  (bind _output_get (set `self.Fpscharacter` fpscharacter))
  (`/Game/blueprint/fpscharacter_BP.Inspecteditem` _output_get
    (:`then`)
    (:`else`
      (`self.Inspectitem`))))

(event `EnhancedInput|/Game/Input/Interact_IA`
  (params (ActionValue :type Boolean) (ElapsedSeconds :type "Float (double-precision)") (TriggeredSeconds :type "Float (double-precision)") (InputAction :type "InputAction Object Reference" :default "/Game/Input/Interact_IA.Interact_IA"))
  ;[1 1 1] If press E -> uninspect
  (:`Started`
    (if (not (`self.Frominventory`))
      (`self.StopInspectionitem`))))

(event `Key|RightMouseButton`
  (params (Key :type "Key Structure"))
  (bind (_iteminformation_itemname _iteminformation_itemdescription _iteminformation_itemimage _iteminformation_item) (break `/Game/blueprint/Inspection/ItemInformation` (`self.iteminformation`)))
  (bind (_iteminformation_itemname_2 _iteminformation_itemdescription_2 _iteminformation_itemimage_2 _iteminformation_item_2 _iteminformation_isstackable_) (break `/Game/blueprint/Inspection/ItemInformation` (`self.iteminformation`)))
  (bind (_iteminformation_itemname_3 _iteminformation_itemdescription_3 _iteminformation_itemimage_3 _iteminformation_item_3) (break `/Game/blueprint/Inspection/ItemInformation` (`self.iteminformation`)))
  (bind _fpscharacter (`self.Fpscharacter`))
  (bind _inventory (`/Game/blueprint/fpscharacter_BP.Inventory` (`self.Fpscharacter`)))
  (bind _inventory_2 (`/Game/blueprint/fpscharacter_BP.Inventory` (`self.Fpscharacter`)))
  ;[1 1 1] Add item in inventory
  (:`Pressed`
    (if (not (`self.Frominventory`))
      (switch `string` (`KismetTextLibrary.Conv_TextToString` _iteminformation_itemname_2)
        (:`Default`
          (if _iteminformation_isstackable_
            (for _array_element _inventory
              (bind _returnvalue (== (`.Item_10_9C7CD19A4DD27ECA2FB2F69834F135BA` (break `/Game/blueprint/Inspection/ItemInformation` _array_element)) _iteminformation_item_3))
              (if _returnvalue
                (break)))
            (if _returnvalue
              (if (> (`KismetArrayLibrary.Array_Length` _inventory) 0)
                (for (_array_element_2 _array_index) _inventory_2
                  (if (== (`.Item_10_9C7CD19A4DD27ECA2FB2F69834F135BA` (break `/Game/blueprint/Inspection/ItemInformation` _array_element_2)) _iteminformation_item)
                    (`KismetArrayLibrary.Array_Set` _inventory_2 _array_index (make `/Game/blueprint/Inspection/ItemInformation` (break `/Game/blueprint/Inspection/ItemInformation` _array_element_2) (`.ItemDescription_4_9A951E574B0A65F764AE3A9557714898` (break `/Game/blueprint/Inspection/ItemInformation` _array_element_2)) (`.Itemimage_7_A82CA1D342013DC59F1F4DBC0C022381` (break `/Game/blueprint/Inspection/ItemInformation` _array_element_2)) (`.Item_10_9C7CD19A4DD27ECA2FB2F69834F135BA` (break `/Game/blueprint/Inspection/ItemInformation` _array_element_2)) (`.isstackable?_13_98E275E24F2997DB3C960FA4C8B6B3A5` (break `/Game/blueprint/Inspection/ItemInformation` _array_element_2)) (+ (`.Number_16_DA1DD91A46C12BB512D368A8BD02D39D` (break `/Game/blueprint/Inspection/ItemInformation` _array_element_2)) 1)))
                    (break)))
                (else
                  (`KismetArrayLibrary.Array_Add` (`/Game/blueprint/fpscharacter_BP.Inventory` (`self.Fpscharacter`)) (`self.iteminformation`) :!label _label)))
              (else
                (goto _label)))
            (else
              (goto _label))))
        (:`Flashlight`
          (set `/Game/blueprint/fpscharacter_BP.Hasflashlight?` true _fpscharacter)
          (`/Game/blueprint/fpscharacter_BP.Toggle flashlight` _fpscharacter))
        (:`Blue Battery`
          (`/Engine/EditorBlueprintResources/StandardMacros.IncrementInt` (`/Game/blueprint/fpscharacter_BP.boxbatteries` _fpscharacter) :!label _label_2
            (:`  `
              (`/Game/blueprint/fpscharacter_BP.Collected Battery` _fpscharacter)
              (goto _label))))
        (:`Green Battery`
          (goto _label_2))
        (:`Red Battery`
          (goto _label_2))
        (:`Yellow Battery`
          (goto _label_2)))
      (`self.StopInspectionitem`)
      (`self.K2_DestroyActor`))))

(event `Closeitem`
  ;[1 1 1] Close Item Event
  (`self.StopInspectionitem`)
  (`self.K2_DestroyActor`))

(event `EnhancedInput|/Game/Input/UseItem_IA`
  (params (ActionValue :type Boolean) (ElapsedSeconds :type "Float (double-precision)") (TriggeredSeconds :type "Float (double-precision)") (InputAction :type "InputAction Object Reference" :default "/Game/Input/UseItem_IA.UseItem_IA"))
  ;[1 1 1] Use Item
  (:`Started`
    (if (`self.Frominventory`)
      (`self.StopInspectionitem`)
      (`/Game/blueprint/fpscharacter_BP.Close Inventory` (`self.Fpscharacter`))
      (`/Game/blueprint/InteractInterface.useitem_f`)
      (`self.K2_DestroyActor`))))

(event `Open item from inventory`
  ;[1 1 1] Open item from inventory Event
  (bind _asfpscharacter_bp (cast `/Game/blueprint/fpscharacter_BP` (`GameplayStatics.GetPlayerCharacter` 0)))
  (bind _output_get (set `self.Fpscharacter` _asfpscharacter_bp))
  (`/Game/blueprint/fpscharacter_BP.Inspecteditem` _output_get
    (:`then`)
    (:`else`
      (`self.Inspectitem`))))

(event `EnhancedInput|/Game/Input/Inventory_IA`
  (params (ActionValue :type Boolean) (ElapsedSeconds :type "Float (double-precision)") (TriggeredSeconds :type "Float (double-precision)") (InputAction :type "InputAction Object Reference" :default "/Game/Input/Inventory_IA.Inventory_IA"))
  ;[1 1 1] Close Inventory
  (:`Started`
    (if (`self.Frominventory`)
      (`self.StopInspectionitem`)
      (`/Game/blueprint/fpscharacter_BP.Close Inventory` (`self.Fpscharacter`))
      (`self.K2_DestroyActor`))))

(fn `Inspectitem`
  (locals (NewLocalVar :type "Vector Structure" :default (0.0 0.0 0.0)))
  (bind _returnvalue (`GameplayStatics.GetPlayerController` 0))
  (bind _returnvalue_2 (`GameplayStatics.GetPlayerCameraManager` 0))
  (bind _fpscharacter (`self.Fpscharacter`))
  (bind (_iteminformation_itemname _iteminformation_itemdescription) (break `/Game/blueprint/Inspection/ItemInformation` (`self.iteminformation`)))
  (set `self.itemoriginallocation` (`SceneComponent.RelativeLocation` (`self.StaticMesh`)))
  (`self.DisableInput` _fpscharacter _returnvalue)
  (`self.EnableInput` _returnvalue)
  (`self.K2_AttachToComponent` (`/Game/blueprint/fpscharacter_BP.Item` _fpscharacter) "None" "SnapToTarget" "SnapToTarget" "KeepRelative")
  (`PrimitiveComponent.SetCollisionEnabled` (`self.StaticMesh`) "NoCollision")
  (set `/Game/blueprint/fpscharacter_BP.Inspecteditem` self (`self.Fpscharacter`))
  (`self.K2_SetActorLocation` (+ (`PlayerCameraManager.GetCameraLocation` _returnvalue_2) (* (`KismetMathLibrary.GetForwardVector` (`PlayerCameraManager.GetCameraRotation` _returnvalue_2)) (`self.inspectiondistance`))))
  (bind _returnvalue_3 (`|CreateWidget` "/Game/UserInterfaces/Item_WB.Item_WB_C" null _iteminformation_itemname _iteminformation_itemdescription))
  (bind _output_get (set `self.itemUI` _returnvalue_3))
  (`UserWidget.AddToViewport` _output_get 0)
  (if (`self.Frominventory`)
    (`Widget.SetVisibility` (`/Game/UserInterfaces/Item_WB.inventorycontrols` _returnvalue_3) "Visible")
    (else
      (`Widget.SetVisibility` (`/Game/UserInterfaces/Item_WB.inspectcontrols` _returnvalue_3) "Visible"))))

(fn `StopInspectionitem`
  (bind _returnvalue (`GameplayStatics.GetPlayerController` 0))
  (bind _itemui (`self.itemUI`))
  (`self.DisableInput` _returnvalue)
  (`self.EnableInput` (`self.Fpscharacter`) _returnvalue)
  (`self.K2_SetActorRelativeLocation` (`self.itemoriginallocation`))
  (`self.K2_DetachFromActor` "KeepRelative")
  (`PrimitiveComponent.SetCollisionEnabled` (`self.StaticMesh`) "QueryAndPhysics")
  (set `/Game/blueprint/fpscharacter_BP.Inspecteditem` null (`self.Fpscharacter`))
  (`/Engine/EditorBlueprintResources/StandardMacros.IsValid` _itemui
    (:`Is Valid`
      (`Widget.RemoveFromParent` _itemui))))

(fn `UserConstructionScript`)
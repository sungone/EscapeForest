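; Interactable battery box that opens the level's Gate_BP once it holds the red, yellow, green and blue batteries.
; The first interaction swings its pivot open 90 degrees in yaw through a DoOnce timeline.
; Every interaction scans the character's inventory by item name, reveals and flags matching batteries, and restarts the loop after each removal.
; With all four flags set, it messages the gate found at BeginPlay.
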(event `self.ReceiveBeginPlay`
  (bind _returnvalue (`GameplayStatics.GetActorOfClass` "/Game/blueprint/Gate_BP.Gate_BP_C"))
  (set `self.gateBP_ref` _returnvalue))

(event `/Game/blueprint/InteractInterface.Interact`
  (params (fpscharacter :type "/Game/blueprint/fpscharacter_BP Object Reference"))
  (`|ExecutionSequence`
    (:`then_0`
      (`/Engine/EditorBlueprintResources/StandardMacros.DoOnce` false
        (:`Completed`
          (bind (_direction _newtrack_0) (`Timeline|Timeline`)
            (:`Update`
              (`SceneComponent.K2_SetRelativeRotation` (`self.pivotpoint`) (`KismetMathLibrary.MakeRotator` 0.0 0.0 (`KismetMathLibrary.Lerp` 0.0 90.0 _newtrack_0)) false false))))))
    (:`then_1`
      (for (_array_element _array_index) (`/Game/blueprint/fpscharacter_BP.Inventory` fpscharacter) :!label _label
        (switch `string` (`KismetTextLibrary.Conv_TextToString` (break `/Game/blueprint/Inspection/ItemInformation` _array_element))
          (:`Blue Battery`
            (`SceneComponent.SetHiddenInGame` (`self.BlueBattery`) false false)
            (set `self.BlueBattery?` true))
          (:`Red Battery`
            (`SceneComponent.SetHiddenInGame` (`self.RedBattery`) false false)
            (set `self.RedBattery?` true))
          (:`Green Battery`
            (`SceneComponent.SetHiddenInGame` (`self.GreenBattery`) false false)
            (set `self.GreenBattery?` true))
          (:`Yellow Battery`
            (`SceneComponent.SetHiddenInGame` (`self.YellowBattery`) false false)
            (set `self.YellowBattery?` true)))
        (`KismetArrayLibrary.Array_RemoveItem` (`/Game/blueprint/fpscharacter_BP.Inventory` fpscharacter) (`|GetArrayItem` (`/Game/blueprint/fpscharacter_BP.Inventory` fpscharacter) _array_index))
        (goto _label))
      ;[1 1 1] 모든 배터리를 모으면
      (if (and (`self.RedBattery?`) (`self.YellowBattery?`) (`self.GreenBattery?`) (`self.BlueBattery?`))
        (message `/Game/blueprint/InteractInterface.Opendoor_f` (`self.gateBP_ref`) true)))))

(fn `UserConstructionScript`)
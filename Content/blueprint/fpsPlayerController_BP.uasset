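; First-person player controller that handles movement and look input for the fpscharacter_BP pawn.
; On BeginPlay it adds the FPS_IMC Enhanced Input mapping context, caches the character and samples its falling state once into Jump.
; Move input drives the pawn along the controller's right and forward vectors, playing the character's footstep timeline while velocity is non-zero and stopping it otherwise or on release.
; Rotate input feeds controller yaw and pitch.
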(event `self.ReceiveBeginPlay`
  (`EnhancedInputSubsystemInterface.AddMappingContext` (subsystem `EnhancedInputLocalPlayerSubsystem`) "/Game/Input/FPS_IMC.FPS_IMC" 0 (struct))
  (bind _asfpscharacter_bp (cast `/Game/blueprint/fpscharacter_BP` (`self.K2_GetPawn`)))
  (set `self.Fpscharacter BP` _asfpscharacter_bp)
  (set `self.Jump?` (`NavMovementComponent.IsFalling` (`Character.CharacterMovement` _asfpscharacter_bp))))

(event `EnhancedInput|/Game/Input/Move_IA`
  (params (ActionValue :type "Vector2D Structure") (ElapsedSeconds :type "Float (double-precision)") (TriggeredSeconds :type "Float (double-precision)") (InputAction :type "InputAction Object Reference" :default "/Game/Input/Move_IA.Move_IA"))
  (bind _returnvalue (`self.K2_GetPawn`))
  (bind _footsteptimeline (`/Game/blueprint/fpscharacter_BP.footsteptimeline` (`self.Fpscharacter BP`)))
  ;[1 1 1] Character Move
  (:`Triggered`
    (`Pawn.AddMovementInput` _returnvalue (`self.GetActorRightVector`) ActionValue_X false)
    (`Pawn.AddMovementInput` _returnvalue (`self.GetActorForwardVector`) ActionValue_Y false)
    ;[1 1 1] footstep sound
    (if (> (`KismetMathLibrary.VSize` (`self.GetVelocity` (`self.K2_GetPawn`))) 0.0)
      (`TimelineComponent.Play` _footsteptimeline)
      (else
        (`TimelineComponent.Stop` _footsteptimeline :!label _label))))
  (:`Completed`
    (goto _label)))

(event `EnhancedInput|/Game/Input/Rotate_IA`
  (params (ActionValue :type "Vector2D Structure") (ElapsedSeconds :type "Float (double-precision)") (TriggeredSeconds :type "Float (double-precision)") (InputAction :type "InputAction Object Reference" :default "/Game/Input/Rotate_IA.Rotate_IA"))
  ;[1 1 1] Character Rotate
  (:`Triggered`
    (`self.AddYawInput` ActionValue_X)
    (`self.AddPitchInput` ActionValue_Y)))

(fn `UserConstructionScript`)
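; First-person player character for a horror game with a Skinwalker monster, handling sprint, jump, line-trace interaction via InteractInterface, HUD and inventory.
; The flashlight spawns as an attached actor, with a looping timer draining battery to the HUD until it switches off.
; Inventory keys and batteries are consumed by events, batteries refilling charge.
; Collected electrical-box batteries escalate Skinwalker speed, then trigger MoveToPlayer; the footstep timeline logic is never triggered.
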(event `self.ReceiveBeginPlay`
  (bind _returnvalue (`GameplayStatics.GetPlayerController` 0))
  ;[1 1 1] Print CrossHair and Information
  (bind _returnvalue_2 (`|CreateWidget` "/Game/UserInterfaces/Player_WB.Player_WB_C"))
  (bind _output_get (set `self.Player HUD` _returnvalue_2))
  (`UserWidget.AddToViewport` _output_get 0)
  ;[1 1 1] Start with light?
  (set `self.Hasflashlight?` true)
  (`self.Toggle flashlight`)
  (bind _returnvalue_3 (`GameplayStatics.GetActorOfClass` "/Game/Monster/Blueprints/Skinwalker_BP.Skinwalker_BP_C"))
  (set `self.skinwalkerref` _returnvalue_3)
  (`WidgetBlueprintLibrary.SetInputMode_GameOnly` _returnvalue)
  (set `PlayerController.bShowMouseCursor` false _returnvalue))

(event `self.ReceiveTick`
  (params (DeltaSeconds :type "Float (single-precision)"))
  (set `self.Speed` (`KismetMathLibrary.VSizeXY` (`MovementComponent.Velocity` (`self.CharacterMovement`)))))

(event `EnhancedInput|/Game/Input/Interact_IA`
  (params (ActionValue :type Boolean) (ElapsedSeconds :type "Float (double-precision)") (TriggeredSeconds :type "Float (double-precision)") (InputAction :type "InputAction Object Reference" :default "/Game/Input/Interact_IA.Interact_IA"))
  (bind _camera (`self.Camera`))
  (bind _returnvalue (`SceneComponent.K2_GetComponentLocation` _camera))
  ;[1 1 1] Message to Item if character press E
  (:`Started`
    (bind _outhit (`KismetSystemLibrary.LineTraceSingle` _returnvalue (+ _returnvalue (* (`KismetMathLibrary.GetForwardVector` (`SceneComponent.K2_GetComponentRotation` _camera)) (`self.InteractDistance`))) "TraceTypeQuery1"))
    (bind (_bblockinghit _binitialoverlap _time _distance _location _impactpoint _normal _impactnormal _physmat _hitactor) (`GameplayStatics.BreakHitResult` _outhit))
    (if (`KismetSystemLibrary.DoesImplementInterface` _hitactor "/Game/blueprint/InteractInterface.InteractInterface_C")
      (message `/Game/blueprint/InteractInterface.Interact` _hitactor self))))

(event `EnhancedInput|/Game/Input/Jump_IA`
  (params (ActionValue :type Boolean) (ElapsedSeconds :type "Float (double-precision)") (TriggeredSeconds :type "Float (double-precision)") (InputAction :type "InputAction Object Reference" :default "/Game/Input/Jump_IA.Jump_IA"))
  ;[1 1 1] Character Jump
  (:`Started`
    (`self.Jump`))
  (:`Completed`
    (`self.StopJumping`)))

(event `EnhancedInput|/Game/Input/Dash_IA`
  (params (ActionValue :type Boolean) (ElapsedSeconds :type "Float (double-precision)") (TriggeredSeconds :type "Float (double-precision)") (InputAction :type "InputAction Object Reference" :default "/Game/Input/Dash_IA.Dash_IA"))
  ;[1 1 1] Character Dash
  (:`Triggered`
    (`TimelineComponent.SetPlayRate` (`self.footsteptimeline`) 1.7)
    (set `CharacterMovementComponent.MaxWalkSpeed` 1000.0 (`self.CharacterMovement`)))
  (:`Completed`
    (`TimelineComponent.SetPlayRate` (`self.footsteptimeline`) 1.7)
    (set `CharacterMovementComponent.MaxWalkSpeed` 600.0 (`self.CharacterMovement`))))

(event `EnhancedInput|/Game/Input/Inventory_IA`
  (params (ActionValue :type Boolean) (ElapsedSeconds :type "Float (double-precision)") (TriggeredSeconds :type "Float (double-precision)") (InputAction :type "InputAction Object Reference" :default "/Game/Input/Inventory_IA.Inventory_IA"))
  (bind _returnvalue (`GameplayStatics.GetPlayerController` 0))
  (bind _inventoryhud (`self.InventoryHUD`))
  ;[1 1 1] Open Inventory
  (:`Started`
    (`self.InventoryHUD`
      (:`then`)
      (:`else`
        (bind _returnvalue_2 (`|CreateWidget` "/Game/UserInterfaces/Inventory_WB.Inventory_WB_C"))
        (set `self.InventoryHUD` _returnvalue_2)
        (for _array_element (`self.Inventory`)
          (`/Game/UserInterfaces/Inventory_WB.Add inventory items` _inventoryhud _array_element))
        (`UserWidget.AddToViewport` _inventoryhud 0)
        (set `PlayerController.bShowMouseCursor` true _returnvalue)
        (`WidgetBlueprintLibrary.SetInputMode_GameAndUIEx` _returnvalue null)
        (`self.DisableInput` self _returnvalue)))))

(event `Close Inventory`
  (bind _returnvalue (`GameplayStatics.GetPlayerController` 0))
  ;[1 1 1] Close Inventory Event
  (`/Engine/EditorBlueprintResources/StandardMacros.IsValid` (`self.InventoryHUD`)
    (:`Is Valid`
      (`Widget.RemoveFromParent` (`self.InventoryHUD`))
      (set `PlayerController.bShowMouseCursor` false _returnvalue)
      (`WidgetBlueprintLibrary.SetInputMode_GameOnly` _returnvalue)
      (set `self.InventoryHUD` null)
      (`self.EnableInput` self _returnvalue))))

(event `EnhancedInput|/Game/Input/Flashlight_IA`
  (params (ActionValue :type Boolean) (ElapsedSeconds :type "Float (double-precision)") (TriggeredSeconds :type "Float (double-precision)") (InputAction :type "InputAction Object Reference" :default "/Game/Input/Flashlight_IA.Flashlight_IA"))
  ;[1 1 1] Handle Flashlight
  (:`Started`
    (if (`self.Hasflashlight?`) :!label _label
      (`/Engine/EditorBlueprintResources/StandardMacros.IsValid` (`self.flashlightref`)
        (:`Is Valid`
          (`GameplayStatics.PlaySoundAtLocation` "/Game/SFX/ButtonOn01.ButtonOn01" (`self.K2_GetActorLocation`) (struct) 1.0 1.0 0.0 null null null null)
          (`self.K2_DestroyActor` (`self.flashlightref`))
          (set `self.flashlightref` null)
          (`Widget.SetVisibility` (`/Game/UserInterfaces/Player_WB.flashlightbox` (`self.Player HUD`)) "Hidden")
          (`KismetSystemLibrary.K2_ClearAndInvalidateTimerHandle` (`self.drain flashlight`)))
        (:`Is Not Valid`
          (`GameplayStatics.PlaySoundAtLocation` "/Game/SFX/ButtonOn01.ButtonOn01" (`self.K2_GetActorLocation`) (struct) 1.0 1.0 0.0 null null null null)
          (bind _returnvalue (`|SpawnActorFromClass` "/Game/blueprint/Flashlight_BP.Flashlight_BP_C" (`SceneComponent.K2_GetComponentToWorld` (`self.Flashlight`)) "Undefined" "MultiplyWithRoot" null null))
          (bind _output_get (set `self.flashlightref` _returnvalue))
          (`self.K2_AttachToComponent` _output_get (`self.Flashlight`) "None" "SnapToTarget" "SnapToTarget" "SnapToTarget" true)
          (`Widget.SetVisibility` (`/Game/UserInterfaces/Player_WB.flashlightbox` (`self.Player HUD`)) "Visible")
          (bind _returnvalue_2 (`KismetSystemLibrary.K2_SetTimerDelegate` (delegate `drain battery`) 0.001 true))
          (set `self.drain flashlight` _returnvalue_2))))))

(event `Toggle flashlight`
  ;[1 1 1] Handle Flashlight
  (goto _label))

(event `drain battery`
  ;[1 1 1] Handle Flashlight
  (bind _output_get (set `self.battery` (- (`self.battery`) (`self.battery drain rate`))))
  (`/Game/UserInterfaces/Player_WB.Update battery` (`self.Player HUD`) _output_get)
  (if (<= _output_get 0.0)
    (`/Game/blueprint/Flashlight_BP.Turn off Flashlight` (`self.flashlightref`))
    (`self.Toggle flashlight`)
    (`KismetSystemLibrary.K2_ClearAndInvalidateTimerHandle` (`self.drain flashlight`))))

(event `Collected Battery`
  (bind _skinwalkerref (`self.skinwalkerref`))
  ;[1 1 1] When electrical box battery is picked up
  (switch `int` (`self.boxbatteries`)
    (:`1`
      (set `/Game/Monster/Blueprints/Skinwalker_BP.Monster Speed` 400.0 _skinwalkerref)
      (`/Game/Monster/Blueprints/Skinwalker_BP.Battery collected` _skinwalkerref :!label _label_2))
    (:`2`
      (set `/Game/Monster/Blueprints/Skinwalker_BP.Monster Speed` 500.0 _skinwalkerref)
      (goto _label_2))
    (:`3`
      (set `/Game/Monster/Blueprints/Skinwalker_BP.Monster Speed` 600.0 _skinwalkerref)
      (goto _label_2))
    (:`4`
      (`/Game/Monster/Blueprints/Skinwalker_BP.Move to Player` _skinwalkerref))))

(event `Use Key`
  (bind _inventory (`self.Inventory`))
  ;[1 1 1] Use Key
  (for (_array_element _array_index) (`self.Inventory`)
    (if (== (`.Item_10_9C7CD19A4DD27ECA2FB2F69834F135BA` (break `/Game/blueprint/Inspection/ItemInformation` _array_element)) "/Game/blueprint/Inspection/Key_BP.Key_BP_C")
      (if (> (`.Number_16_DA1DD91A46C12BB512D368A8BD02D39D` (break `/Game/blueprint/Inspection/ItemInformation` _array_element)) 1)
        (`KismetArrayLibrary.Array_Set` (`self.Inventory`) _array_index (make `/Game/blueprint/Inspection/ItemInformation` (break `/Game/blueprint/Inspection/ItemInformation` _array_element) (`.ItemDescription_4_9A951E574B0A65F764AE3A9557714898` (break `/Game/blueprint/Inspection/ItemInformation` _array_element)) (`.Itemimage_7_A82CA1D342013DC59F1F4DBC0C022381` (break `/Game/blueprint/Inspection/ItemInformation` _array_element)) (`.Item_10_9C7CD19A4DD27ECA2FB2F69834F135BA` (break `/Game/blueprint/Inspection/ItemInformation` _array_element)) (`.isstackable?_13_98E275E24F2997DB3C960FA4C8B6B3A5` (break `/Game/blueprint/Inspection/ItemInformation` _array_element)) (- (`.Number_16_DA1DD91A46C12BB512D368A8BD02D39D` (break `/Game/blueprint/Inspection/ItemInformation` _array_element)) 1)))
        (else
          (`KismetArrayLibrary.Array_RemoveItem` _inventory (`|GetArrayItem` _inventory _array_index)))))))

(event `Use Battery`
  (bind _inventory (`self.Inventory`))
  ;[1 1 1] Use Battery
  (for (_array_element _array_index) (`self.Inventory`)
    (if (== (`.Item_10_9C7CD19A4DD27ECA2FB2F69834F135BA` (break `/Game/blueprint/Inspection/ItemInformation` _array_element)) "/Game/blueprint/Inspection/BatteryInv_BP.BatteryInv_BP_C")
      (if (> (`.Number_16_DA1DD91A46C12BB512D368A8BD02D39D` (break `/Game/blueprint/Inspection/ItemInformation` _array_element)) 1)
        (`KismetArrayLibrary.Array_Set` (`self.Inventory`) _array_index (make `/Game/blueprint/Inspection/ItemInformation` (break `/Game/blueprint/Inspection/ItemInformation` _array_element) (`.ItemDescription_4_9A951E574B0A65F764AE3A9557714898` (break `/Game/blueprint/Inspection/ItemInformation` _array_element)) (`.Itemimage_7_A82CA1D342013DC59F1F4DBC0C022381` (break `/Game/blueprint/Inspection/ItemInformation` _array_element)) (`.Item_10_9C7CD19A4DD27ECA2FB2F69834F135BA` (break `/Game/blueprint/Inspection/ItemInformation` _array_element)) (`.isstackable?_13_98E275E24F2997DB3C960FA4C8B6B3A5` (break `/Game/blueprint/Inspection/ItemInformation` _array_element)) (- (`.Number_16_DA1DD91A46C12BB512D368A8BD02D39D` (break `/Game/blueprint/Inspection/ItemInformation` _array_element)) 1)))
        (set `self.battery` 1.0)
        (else
          (set `self.battery` 1.0)
          (`KismetArrayLibrary.Array_RemoveItem` _inventory (`|GetArrayItem` _inventory _array_index)))))))

(fn `UserConstructionScript`)
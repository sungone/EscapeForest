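; Door actor that swings open when the player interacts, optionally requiring a matching key from the character's inventory.
; Interact opens an unlocked door directly; a locked one opens only for inventory entries matching KeyToOpenDoor.
; OpenDoor plays a timeline that lerps the mesh's yaw to a quarter turn, with no closing logic.
; Both opening paths call UseKey on the FPS character cached at BeginPlay, even when the door is unlocked.
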(event `self.ReceiveBeginPlay`
  (bind _returnvalue (`GameplayStatics.GetActorOfClass` "/Game/blueprint/fpscharacter_BP.fpscharacter_BP_C"))
  (set `self.fpscharacter_ref` _returnvalue))

(event `Open Door`
  ;[1 1 1] Open Door Animation
  (bind (_direction _door_opentrack) (`Timeline|door open timeline`)
    (:`Update`
      (`SceneComponent.K2_SetRelativeRotation` (`self.Door`) (`KismetMathLibrary.MakeRotator` 0.0 0.0 (`KismetMathLibrary.Lerp` 0.0 -90.0 _door_opentrack)) false false))))

(event `/Game/blueprint/InteractInterface.Interact`
  (params (fpscharacter :type "/Game/blueprint/fpscharacter_BP Object Reference"))
  ;[1 1 1] Interact
  (if (`self.Isdoorlocked?`)
    (for _array_element (`/Game/blueprint/fpscharacter_BP.Inventory` fpscharacter)
      (if (== (`.Item_10_9C7CD19A4DD27ECA2FB2F69834F135BA` (break `/Game/blueprint/Inspection/ItemInformation` _array_element)) (`self.KeyToOpenDoor`))
        (`self.Open Door`)
        (`/Game/blueprint/fpscharacter_BP.Use Key` (`self.fpscharacter_ref`))))
    (else
      (`self.Open Door`)
      (`/Game/blueprint/fpscharacter_BP.Use Key` (`self.fpscharacter_ref`)))))

(fn `UserConstructionScript`)
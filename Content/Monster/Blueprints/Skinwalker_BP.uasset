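; Skinwalker monster AI that roams the navmesh, hunts the player and triggers game over on contact.
; Pawn sensing starts a chase with fading music; a retriggerable delay returns it to random roaming after sight is lost.
; External events can force a chase or reapply MonsterSpeed upon battery collection.
; Hitting the player destroys their flashlight, blends the camera to the monster, plays an attack montage and shows the GameOver widget.
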(event `Randomlyroam`
  (bind _randomlocation (`NavigationSystemV1.K2_GetRandomLocationInNavigableRadius` (`self.K2_GetActorLocation`) 3000.0 null null :!label _label))
  (`|AIMoveTo` self _randomlocation null
    (:`then`
      _)
    (:`OnSuccess`
      _))
  (`KismetSystemLibrary.Delay` 4.0)
  (if (not (`self.seeplayer?`))
    (`self.Randomlyroam`)))

(event `self.ReceiveBeginPlay`
  (set `CharacterMovementComponent.MaxWalkSpeed` (`self.Monster Speed`) (`self.CharacterMovement`))
  (goto _label))

(event `self.PawnSensing.OnSeePawn`
  (params (Pawn :type "Pawn Object Reference"))
  (bind _returnvalue (`GameplayStatics.GetPlayerCharacter` 0))
  ;[1 1 1] On see Player
  (if (== Pawn _returnvalue)
    (`|ExecutionSequence`
      (:`then_0`
        (set `self.seeplayer?` true)
        (`|AIMoveTo` self (0.0 0.0 0.0) _returnvalue
          (:`then`
            (`self.chasesequence`
              (:`then`)
              (:`else`
                (bind _returnvalue_2 (`GameplayStatics.SpawnSound2D` "/Game/Sounds/chasesequence.chasesequence" 1.0 1.0 0.0 null))
                (bind _output_get (set `self.chasesequence` _returnvalue_2))
                (`AudioComponent.FadeIn` _output_get 3.0 1.0 0.0 "Linear"))))))
      (:`then_1`
        (`KismetSystemLibrary.RetriggerableDelay` 1.5)
        (set `self.seeplayer?` false)
        (`self.Randomlyroam`)
        (bind _chasesequence (`self.chasesequence`)
          (:`then`
            (`AudioComponent.FadeOut` _chasesequence 1.5 0.0 "Linear")
            (`KismetSystemLibrary.Delay` 1.0)
            (set `self.chasesequence` null))
          (:`else`))))))

(event `Battery collected`
  ;[1 1 1] Monster Speed highly if player get battery
  (set `CharacterMovementComponent.MaxWalkSpeed` (`self.Monster Speed`) (`self.CharacterMovement`)))

(event `self.CapsuleComponent.OnComponentHit`
  (params (HitComponent :type "PrimitiveComponent Object Reference") (OtherActor :type "Actor Object Reference") (OtherComp :type "PrimitiveComponent Object Reference") (NormalImpulse :type "Vector Structure") (Hit :type "HitResult Structure (by ref)"))
  ;[1 1 1] Attack Player Animation
  (bind _asfpscharacter_bp (cast `/Game/blueprint/fpscharacter_BP` OtherActor))
  (`/Engine/EditorBlueprintResources/StandardMacros.DoOnce` false
    (:`Completed`
      (`self.K2_DestroyActor` (`/Game/blueprint/fpscharacter_BP.flashlightref` _asfpscharacter_bp))
      (`PlayerController.SetViewTargetWithBlend` (`GameplayStatics.GetPlayerController` 0) self 0.3 "VTBlend_Linear" 0.0 false)
      (bind _returnvalue (`self.PlayAnimMontage` "/Game/Monster/Animation/monsterattack_Montage.monsterattack_Montage"))
      (`KismetSystemLibrary.Delay` (- _returnvalue 1.2))
      (bind _returnvalue_2 (`|CreateWidget` "/Game/UserInterfaces/GameOver_WB.GameOver_WB_C"))
      (`UserWidget.AddToViewport` _returnvalue_2 0))))

(event `Move to Player`
  ;[1 1 1] Move To Player
  (set `self.seeplayer?` true)
  (`|AIMoveTo` self (0.0 0.0 0.0) (`GameplayStatics.GetPlayerCharacter` 0)))

(fn `UserConstructionScript`)